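; Note is a greyboxing Blueprint that displays multi-line text in the level.
; Its construction script adds one Text Render component per entry in the Textrows array, stacking each row below the previous one at a fixed vertical spacing.
; Every row shares the alignment and color set by the TextAlignment and TextColor variables.
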(fn ConstructionScript
  (for (_array_element _array_index) (Variables|Text|GetTextrows)
    (bind _returnvalue (AddComponent|AddTextRenderComponent false))
    (Rendering|Components|TextRender|SetText _returnvalue _array_element)
    (Transformation|SetRelativeLocation _returnvalue (Math|Vector|MakeVector 0.0 0.0 (* _array_index -2e+01)) false)
    (Rendering|Components|TextRender|SetHorizontalAlignment _returnvalue (Variables|Text|GetTextAlignment))
    (Rendering|Components|TextRender|SetTextRenderColor _returnvalue (Math|Conversions|ToColor(LinearColor) (Variables|Text|GetTextColor)))))